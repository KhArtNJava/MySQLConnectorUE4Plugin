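; SQL_TESTER is a test Blueprint that exercises a MySQL connection on BeginPlay.
; After a delay, it connects using credentials from a DatabaseInfo object, then runs a timed loop capped by DoN.
; Each pass opens a transaction, inserts a random user with an MD5-hashed password, prints the user table and commits, rolling back on error.
; EndPlay closes the connection.
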(event EventBeginPlay
  (Utilities|FlowControl|Delay 5.0)
  (bind _returnvalue (Game|ConstructObjectfromClass "/MySQLConnectorUE4Plugin/Blueprints/Information/DatabaseInfo.DatabaseInfo_C" self))
  (bind (_address _user _password _database) (Default|GetDBLoginData _returnvalue))
  (bind (_connection _errormessage) (Utilities|MySQLConnect _address _user _password _database)
    (:Success
      (Utilities|FlowControl|Delay 5.0 :!label _label)
      (Utilities|FlowControl|DoN 10
        (:Exit
          (Utilities|FlowControl|Sequence
            (:then_0
              (Utilities|MySQLStartTransaction _connection
                (:Success
                  (Utilities|MySQLExecuteQuery (Utilities|String|Append "INSERT INTO ar.user 
( 
	id, 
    name, 
    password, 
    created) 
VALUES 
( 
	default, 
    '" (Utilities|String|MakeLiteralString (Utilities|String|ToString(Float) (Math|Random|RandomFloat))) "',md5('" (Utilities|String|MakeLiteralString (Utilities|String|ToString(Float) (Math|Random|RandomFloat))) "'), 
    now() 
);") _connection
                    (:Success
                      (bind _result_rows (Utilities|MySQLExecuteQuerywithResult "select * from user;" _connection)
                        (:Success
                          (for (_array_element _array_index) _result_rows
                            (Development|PrintString (Utilities|String|ToString(Integer) _array_index) true true "(R=1.000000,G=0.000000,B=0.052997,A=1.000000)")
                            ;[1 1 1] QueryResults
                            (for (_array_element_2 _array_index_2) (.fields _array_element)
                              (Development|PrintString (Utilities|String|Append (Utilities|String|ToString(Integer) _array_index_2) " : " (.key _array_element_2) " : " (.value _array_element_2)))))
                          (Utilities|MySQLCommit _connection
                            (:Error
                              _)))
                        (:Error
                          _)))
                    (:Error
                      _)))
                (:Error
                  _))
              (Utilities|MySQLRollback _connection))
            (:then_1
              (goto _label))))))
    (:Error
      (Development|PrintString (Utilities|String|Append "Failed to connect to DB: " _errormessage) true true "(R=1.000000,G=0.000000,B=0.000000,A=1.000000)"))))

(event EventEndPlay
  (params (EndPlayReason :type EEndPlayReason%20Enum :default "Destroyed"))
  (bind _errormessage (Utilities|MySQLClose (stale EventBeginPlay _connection))
    (:Success
      (Development|PrintString "Closed Connection"))
    (:Error
      (Development|PrintString _errormessage true true "(R=1.000000,G=0.000000,B=0.000000,A=1.000000)"))))

(fn ConstructionScript)